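; BP_PlatformWallSnap is a rhythm game platform wall that snaps between two positions on clock input and respawns the player on contact with its box.
; BeginPlay stores the start location and an end location offset by Distance.
; Clock input for a matching instrument type teleports the root to either location according to its On state, without sweep or interpolation.
; Player overlap with the box calls SpawnPlayer on BP_SpawnManager.
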(event `self.ReceiveBeginPlay`
  (set `self.StartLocation` (`SceneComponent.K2_GetComponentLocation` (`self.DefaultSceneRoot`)))
  (set `self.EndLocation` (+ (`self.StartLocation`) (`self.Distance`))))

(event `self.RecieveClockInput`
  (params (InstrumentType :type "/Game/RhythmGame/Blueprints/Enumeration/E_InstrumentType Enum" :default "NewEnumerator0") (`On?` :type Boolean))
  (if (`KismetStringLibrary.EqualEqual_StrStr` (`|GetEnumeratorNameAsString` InstrumentType) (`|GetEnumeratorNameAsString` (`self.InstrumentType`)))
    (if `On?`
      (`SceneComponent.K2_SetWorldLocation` (`self.DefaultSceneRoot`) (`self.EndLocation`) false false)
      (else
        (`SceneComponent.K2_SetWorldLocation` (`self.DefaultSceneRoot`) (`self.StartLocation`) false false)))))

(event `self.Box.OnComponentBeginOverlap`
  (params (OverlappedComponent :type "PrimitiveComponent Object Reference") (OtherActor :type "Actor Object Reference") (OtherComp :type "PrimitiveComponent Object Reference") (OtherBodyIndex :type Integer) (bFromSweep :type Boolean) (SweepResult :type "HitResult Structure (by ref)"))
  (if (== OtherActor (`GameplayStatics.GetPlayerPawn` 0))
    (bind _returnvalue (`GameplayStatics.GetActorOfClass` "/Game/RhythmGame/Blueprints/Spawning/BP_SpawnManager.BP_SpawnManager_C"))
    (`/Game/RhythmGame/Blueprints/Spawning/BP_SpawnManager.SpawnPlayer` _returnvalue)))

(fn `UserConstructionScript`)