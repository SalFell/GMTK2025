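; BP_PlatformBlinking is a rhythm-game platform that blinks between solid and passable in response to clock input.
; On a matching InstrumentType signal, it swaps the static mesh material and toggles its collision between QueryAndPhysics and NoCollision.
; A separate Box trigger calls SpawnPlayer on BP_SpawnManager when the player pawn overlaps it, independent of the blink state.
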(event `/Game/RhythmGame/Blueprints/Interfaces/BPI_PlatformFunctionality.RecieveClockInput`
  (params (InstrumentType :type "/Game/RhythmGame/Blueprints/Enumeration/E_InstrumentType Enum" :default "NewEnumerator0") (`On?` :type Boolean))
  (bind _staticmesh (`self.StaticMesh`))
  (bind _staticmesh_2 (`self.StaticMesh`))
  (if (`|EnumEquality` InstrumentType (`self.InstrumentType`))
    (if `On?`
      (`PrimitiveComponent.SetMaterial` _staticmesh 0 (`self.OnMaterial`))
      (`PrimitiveComponent.SetCollisionEnabled` _staticmesh "QueryAndPhysics")
      (else
        (`PrimitiveComponent.SetMaterial` _staticmesh_2 0 (`self.OffMaterial`))
        (`PrimitiveComponent.SetCollisionEnabled` _staticmesh_2 "NoCollision")))))

(event `self.Box.OnComponentBeginOverlap`
  (params (OverlappedComponent :type "PrimitiveComponent Object Reference") (OtherActor :type "Actor Object Reference") (OtherComp :type "PrimitiveComponent Object Reference") (OtherBodyIndex :type Integer) (bFromSweep :type Boolean) (SweepResult :type "HitResult Structure (by ref)"))
  (if (== OtherActor (`GameplayStatics.GetPlayerPawn` 0))
    (bind _returnvalue (`GameplayStatics.GetActorOfClass` "/Game/RhythmGame/Blueprints/Spawning/BP_SpawnManager.BP_SpawnManager_C"))
    (`/Game/RhythmGame/Blueprints/Spawning/BP_SpawnManager.SpawnPlayer` _returnvalue)))

(fn `UserConstructionScript`)