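; Moving wall for a rhythm game that slides between its start position and an offset end point in response to clock input for its instrument type.
; On BeginPlay, a macro sets the end point from a world-axis direction and distance, and the timeline play rate is derived from BPM and duration in beats.
; A matching "on" input plays the lerp timeline from the start, and "off" reverses it.
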(event `self.ReceiveBeginPlay`
  (set `self.StartPos` (`self.K2_GetActorLocation`))
  (`self.SwitchPlatformDirection`
    (:`then`
      _)
    (:`then2`
      _)
    (:`then3`
      _)
    (:`then4`
      _)
    (:`then5`
      _)
    (:`then6`
      _))
  (`TimelineComponent.SetPlayRate` (`self.MovePlatformTimeline`) (/ 1.0 (* (`self.MoveDurationInBeats`) (/ (`self.BPM`) 60.0)))))

(event `/Game/RhythmGame/Blueprints/Interfaces/BPI_PlatformFunctionality.RecieveClockInput`
  (params (InstrumentType :type "/Game/RhythmGame/Blueprints/Enumeration/E_InstrumentType Enum" :default "NewEnumerator0") (`On?` :type Boolean))
  (if (`|EnumEquality` InstrumentType (`self.Instrument Type`))
    (if `On?`
      (bind (_direction _progress) (`Timeline|MovePlatformTimeline` :!via `PlayFromStart` :!label _label)
        (:`Update`
          (`self.K2_SetActorLocation` (`KismetMathLibrary.VLerp` (`self.StartPos`) (`self.EndPos`) _progress))))
      (else
        (goto _label :!via `Reverse`)))))

(fn `UserConstructionScript`)