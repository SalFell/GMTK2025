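; Quartz-driven music manager for a rhythm game that layers six looping instrument stems and sends their bar pulses to platforms.
; All stems are queued quantized to the bar on one clock, with all but the kick muted, and re-queued after a set bar count.
; A checkpoint call opens a gate so the chosen instrument unmutes on the next bar.
; Each bar, active instruments message every BPI_PlatformFunctionality actor.
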(event `BarEvents`
  (params (ClockName :type Name) (QuantizationType :type "EQuartzCommandQuantization Enum" :default "Bar") (NumBars :type Integer) (Beat :type Integer) (BeatFraction :type "Float (single-precision)"))
  ; Count & Retrigger
  (`KismetSystemLibrary.PrintString` (`KismetStringLibrary.Conv_IntToString` NumBars))
  (if (== NumBars (`self.NumofBars`))
    (`self.QueueMusic`)
    (`QuartzClockHandle.ResetTransportQuantized` :`self` (`self.QuartzClock`) :`InQuantizationBoundary` (make `QuartzQuantizationBoundary` "Bar" 1.0 "CurrentTimeRelative"))))

(event `self.ReceiveBeginPlay`
  ; Setup Quartz Clock
  (bind _returnvalue (`QuartzSubsystem.CreateNewClock` (subsystem `QuartzSubsystem`) "QuartzMaster" (make `QuartzClockSettings` (make `QuartzTimeSignature` 4)) false true))
  (bind _output_get (set `self.QuartzClock` _returnvalue))
  (bind _clockhandle (`QuartzClockHandle.SetBeatsPerMinute` :`self` _output_get :`BeatsPerMinute` 120.0))
  (bind _clockhandle_2 (`QuartzClockHandle.SubscribeToQuantizationEvent` _clockhandle "Bar" (`|CreateDelegate` :!event `BarEvents`)))
  (bind _clockhandle_3 (`QuartzClockHandle.SubscribeToQuantizationEvent` _clockhandle_2 "Bar" (`|CreateDelegate` :!event `KickDrumBar`)))
  (bind _clockhandle_4 (`QuartzClockHandle.SubscribeToQuantizationEvent` _clockhandle_3 "Bar" (`|CreateDelegate` :!event `HiHatBar`)))
  (bind _clockhandle_5 (`QuartzClockHandle.SubscribeToQuantizationEvent` _clockhandle_4 "Bar" (`|CreateDelegate` :!event `ClapBar`)))
  (bind _clockhandle_6 (`QuartzClockHandle.SubscribeToQuantizationEvent` _clockhandle_5 "Bar" (`|CreateDelegate` :!event `LeadBar`)))
  (bind _clockhandle_7 (`QuartzClockHandle.SubscribeToQuantizationEvent` _clockhandle_6 "Bar" (`|CreateDelegate` :!event `KeysBar`)))
  (bind _clockhandle_8 (`QuartzClockHandle.SubscribeToQuantizationEvent` _clockhandle_7 "Bar" (`|CreateDelegate` :!event `BrassBar`)))
  (`QuartzClockHandle.SubscribeToQuantizationEvent` _clockhandle_8 "Bar" (`|CreateDelegate` :!event `StartInstrumentOnBar`))
  (`self.QueueMusic`))

(event `QueueMusic`
  ; Queue Music
  ;; KickDrum
  (bind _returnvalue (`GameplayStatics.CreateSound2D` "/Game/RhythmGame/Audio/KickDrum.KickDrum" 1.0 1.0 0.0 null))
  (`AudioComponent.SetVolumeMultiplier` _returnvalue 1.0)
  (`AudioComponent.PlayQuantized` _returnvalue (`self.QuartzClock`) (make `QuartzQuantizationBoundary` "Bar" 1.0 "TransportRelative") (delegate `CustomEvent`) 0.0 0.0 1.0 "Linear")
  ;; HiHat
  (bind _returnvalue_2 (`GameplayStatics.CreateSound2D` "/Game/RhythmGame/Audio/HiHat.HiHat" 1.0 1.0 0.0 null)) ; Make sure sound is set to Play When Silent
  (`AudioComponent.SetVolumeMultiplier` _returnvalue_2 0.0)
  (`AudioComponent.PlayQuantized` _returnvalue_2 (`self.QuartzClock`) (make `QuartzQuantizationBoundary` "Bar" 1.0 "TransportRelative") (delegate `CustomEvent_0`) 0.0 0.0 1.0 "Linear")
  ;; Clap
  (bind _returnvalue_3 (`GameplayStatics.CreateSound2D` "/Game/RhythmGame/Audio/Clap.Clap" 1.0 1.0 0.0 null)) ; Make sure sound is set to Play When Silent
  (`AudioComponent.SetVolumeMultiplier` _returnvalue_3 0.0)
  (`AudioComponent.PlayQuantized` _returnvalue_3 (`self.QuartzClock`) (make `QuartzQuantizationBoundary` "Bar" 1.0 "TransportRelative") (delegate `CustomEvent_1`) 0.0 0.0 1.0 "Linear")
  ;; Lead
  (bind _returnvalue_4 (`GameplayStatics.CreateSound2D` "/Game/RhythmGame/Audio/Lead.Lead" 1.0 1.0 0.0 null)) ; Make sure sound is set to Play When Silent
  (`AudioComponent.SetVolumeMultiplier` _returnvalue_4 0.0)
  (`AudioComponent.PlayQuantized` _returnvalue_4 (`self.QuartzClock`) (make `QuartzQuantizationBoundary` "Bar" 1.0 "TransportRelative") (delegate `CustomEvent_2`) 0.0 0.0 1.0 "Linear")
  ;; Keys
  (bind _returnvalue_5 (`GameplayStatics.CreateSound2D` "/Game/RhythmGame/Audio/Keys.Keys" 1.0 1.0 0.0 null)) ; Make sure sound is set to Play When Silent
  (`AudioComponent.SetVolumeMultiplier` _returnvalue_5 0.0)
  (`AudioComponent.PlayQuantized` _returnvalue_5 (`self.QuartzClock`) (make `QuartzQuantizationBoundary` "Bar" 1.0 "TransportRelative") (delegate `CustomEvent_3`) 0.0 0.0 1.0 "Linear")
  ;; Brass
  (bind _returnvalue_6 (`GameplayStatics.CreateSound2D` "/Game/RhythmGame/Audio/Brass.Brass" 1.0 1.0 0.0 null)) ; Make sure sound is set to Play When Silent
  (`AudioComponent.SetVolumeMultiplier` _returnvalue_6 0.0)
  (`AudioComponent.PlayQuantized` _returnvalue_6 (`self.QuartzClock`) (make `QuartzQuantizationBoundary` "Bar" 1.0 "TransportRelative") (delegate `CustomEvent_4`) 0.0 0.0 1.0 "Linear"))

(event `CustomEvent_0`
  (params (EventType :type "EQuartzCommandDelegateSubType Enum" :default "CommandOnFailedToQueue") (Name :type Name))
  ; Queue Music
  (switch `EQuartzCommandDelegateSubType` EventType
    (:`CommandOnStarted`
      (bind _output_get (set `self.HiHat` (stale `QueueMusic` _returnvalue_2)))
      (`AudioComponent.SetVolumeMultiplier` _output_get (`self.HiHatVolume`)))))

(event `CustomEvent_2`
  (params (EventType :type "EQuartzCommandDelegateSubType Enum" :default "CommandOnFailedToQueue") (Name :type Name))
  ; Queue Music
  (switch `EQuartzCommandDelegateSubType` EventType
    (:`CommandOnStarted`
      (bind _output_get (set `self.Lead` (stale `QueueMusic` _returnvalue_4)))
      (`AudioComponent.SetVolumeMultiplier` _output_get (`self.LeadVolume`)))))

(event `CustomEvent_1`
  (params (EventType :type "EQuartzCommandDelegateSubType Enum" :default "CommandOnFailedToQueue") (Name :type Name))
  ; Queue Music
  (switch `EQuartzCommandDelegateSubType` EventType
    (:`CommandOnStarted`
      (bind _output_get (set `self.Clap` (stale `QueueMusic` _returnvalue_3)))
      (`AudioComponent.SetVolumeMultiplier` _output_get (`self.ClapVolume`)))))

(event `CustomEvent_3`
  (params (EventType :type "EQuartzCommandDelegateSubType Enum" :default "CommandOnFailedToQueue") (Name :type Name))
  ; Queue Music
  (switch `EQuartzCommandDelegateSubType` EventType
    (:`CommandOnStarted`
      (bind _output_get (set `self.Keys` (stale `QueueMusic` _returnvalue_5)))
      (`AudioComponent.SetVolumeMultiplier` _output_get (`self.KeysVolume`)))))

(event `CustomEvent_4`
  (params (EventType :type "EQuartzCommandDelegateSubType Enum" :default "CommandOnFailedToQueue") (Name :type Name))
  ; Queue Music
  (switch `EQuartzCommandDelegateSubType` EventType
    (:`CommandOnQueued`
      (`/Engine/EditorBlueprintResources/StandardMacros.DoOnce` false
        (:`Completed`
          (`QuartzClockHandle.StartClock` (`self.QuartzClock`)))))
    (:`CommandOnStarted`
      (bind _output_get (set `self.Brass` (stale `QueueMusic` _returnvalue_6)))
      (`AudioComponent.SetVolumeMultiplier` _output_get (`self.BrassVolume`)))))

(event `CustomEvent`
  (params (EventType :type "EQuartzCommandDelegateSubType Enum" :default "CommandOnFailedToQueue") (Name :type Name))
  ; Queue Music
  (switch `EQuartzCommandDelegateSubType` EventType
    (:`CommandOnStarted`
      (bind _output_get (set `self.KickDrum` (stale `QueueMusic` _returnvalue)))
      (`AudioComponent.SetVolumeMultiplier` _output_get (`self.KickDrumVolume`)))))

(event `StartInstrument`
  (params (InstrumentType :type "/Game/RhythmGame/Blueprints/Enumeration/E_InstrumentType Enum" :default "NewEnumerator0"))
  ; Called from checkpoint
  (`self.OpenGate` InstrumentType))

(event `KickDrumBar`
  (params (ClockName :type Name) (QuantizationType :type "EQuartzCommandQuantization Enum" :default "Bar") (NumBars :type Integer) (Beat :type Integer) (BeatFraction :type "Float (single-precision)"))
  (bind _outactors (`GameplayStatics.GetAllActorsWithInterface` "/Game/RhythmGame/Blueprints/Interfaces/BPI_PlatformFunctionality.BPI_PlatformFunctionality_C"))
  (for _array_element _outactors
    (message `/Game/RhythmGame/Blueprints/Interfaces/BPI_PlatformFunctionality.RecieveClockInput` _array_element (`self.KickDrumSend`))))

(event `StartInstrumentOnBar`
  (params (ClockName :type Name) (QuantizationType :type "EQuartzCommandQuantization Enum" :default "Bar") (NumBars :type Integer) (Beat :type Integer) (BeatFraction :type "Float (single-precision)"))
  (`/Engine/EditorBlueprintResources/StandardMacros.Gate` true :!label _label
    (:`Exit`
      (`|ExecutionSequence`
        (:`then_0`
          (switch `/Game/RhythmGame/Blueprints/Enumeration/E_InstrumentType` (stale `OpenGate` InstrumentType)
            (:`NewEnumerator1`
              (`AudioComponent.SetVolumeMultiplier` (`self.HiHat`) 1.0)
              (set `self.HiHatVolume` 1.0)
              (set `self.HiHatOn?` true))
            (:`NewEnumerator2`
              (`AudioComponent.SetVolumeMultiplier` (`self.Clap`) 1.0)
              (set `self.ClapVolume` 1.0)
              (set `self.ClapOn?` true))
            (:`NewEnumerator3`
              (`AudioComponent.SetVolumeMultiplier` (`self.Lead`) 1.0)
              (set `self.LeadVolume` 1.0)
              (set `self.LeadOn?` true))
            (:`NewEnumerator4`
              (`AudioComponent.SetVolumeMultiplier` (`self.Keys`) 1.0)
              (set `self.KeysVolume` 1.0)
              (set `self.KeysOn?` true))
            (:`NewEnumerator5`
              (`AudioComponent.SetVolumeMultiplier` (`self.Brass`) 1.0)
              (set `self.BrassVolume` 1.0)
              (set `self.BrassOn?` true))))
        (:`then_1`
          (goto _label :!via `Close`))))))

(event `HiHatBar`
  (params (ClockName :type Name) (QuantizationType :type "EQuartzCommandQuantization Enum" :default "Bar") (NumBars :type Integer) (Beat :type Integer) (BeatFraction :type "Float (single-precision)"))
  (if (`self.HiHatOn?`)
    (bind _outactors (`GameplayStatics.GetAllActorsWithInterface` "/Game/RhythmGame/Blueprints/Interfaces/BPI_PlatformFunctionality.BPI_PlatformFunctionality_C"))
    (for _array_element _outactors
      (message `/Game/RhythmGame/Blueprints/Interfaces/BPI_PlatformFunctionality.RecieveClockInput` _array_element (`self.HiHatSend`)))))

(event `OpenGate`
  (params (InstrumentType :type "/Game/RhythmGame/Blueprints/Enumeration/E_InstrumentType Enum" :default "NewEnumerator0"))
  (goto _label :!via `Open`))

(event `ClapBar`
  (params (ClockName :type Name) (QuantizationType :type "EQuartzCommandQuantization Enum" :default "Bar") (NumBars :type Integer) (Beat :type Integer) (BeatFraction :type "Float (single-precision)"))
  (if (`self.ClapOn?`)
    (bind _outactors (`GameplayStatics.GetAllActorsWithInterface` "/Game/RhythmGame/Blueprints/Interfaces/BPI_PlatformFunctionality.BPI_PlatformFunctionality_C"))
    (for _array_element _outactors
      (message `/Game/RhythmGame/Blueprints/Interfaces/BPI_PlatformFunctionality.RecieveClockInput` _array_element (`self.ClapSend`)))))

(event `LeadBar`
  (params (ClockName :type Name) (QuantizationType :type "EQuartzCommandQuantization Enum" :default "Bar") (NumBars :type Integer) (Beat :type Integer) (BeatFraction :type "Float (single-precision)"))
  (if (`self.LeadOn?`)
    (bind _outactors (`GameplayStatics.GetAllActorsWithInterface` "/Game/RhythmGame/Blueprints/Interfaces/BPI_PlatformFunctionality.BPI_PlatformFunctionality_C"))
    (for _array_element _outactors
      (message `/Game/RhythmGame/Blueprints/Interfaces/BPI_PlatformFunctionality.RecieveClockInput` _array_element (`self.LeadSend`)))))

(event `KeysBar`
  (params (ClockName :type Name) (QuantizationType :type "EQuartzCommandQuantization Enum" :default "Bar") (NumBars :type Integer) (Beat :type Integer) (BeatFraction :type "Float (single-precision)"))
  (if (`self.KeysOn?`)
    (bind _outactors (`GameplayStatics.GetAllActorsWithInterface` "/Game/RhythmGame/Blueprints/Interfaces/BPI_PlatformFunctionality.BPI_PlatformFunctionality_C"))
    (for _array_element _outactors
      (message `/Game/RhythmGame/Blueprints/Interfaces/BPI_PlatformFunctionality.RecieveClockInput` _array_element (`self.KeysSend`)))))

(event `BrassBar`
  (params (ClockName :type Name) (QuantizationType :type "EQuartzCommandQuantization Enum" :default "Bar") (NumBars :type Integer) (Beat :type Integer) (BeatFraction :type "Float (single-precision)"))
  (if (`self.BrassOn?`)
    (bind _outactors (`GameplayStatics.GetAllActorsWithInterface` "/Game/RhythmGame/Blueprints/Interfaces/BPI_PlatformFunctionality.BPI_PlatformFunctionality_C"))
    (for _array_element _outactors
      (message `/Game/RhythmGame/Blueprints/Interfaces/BPI_PlatformFunctionality.RecieveClockInput` _array_element (`self.BrassSend`)))))

(fn `UserConstructionScript`)