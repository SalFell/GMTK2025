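; BP_Blinking_Platform is a rhythm game platform that switches between a solid visible state and a non-colliding invisible state.
; Its Visible event applies OnMaterial to the static mesh and enables query and physics collision, while Invisible applies OffMaterial and disables collision.
; The Blueprint contains no timing logic of its own and never calls either event itself.
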(event `/Game/RhythmGame/Blueprints/Interfaces/BPI_BlinkingPlatform.Visible`
  (`PrimitiveComponent.SetMaterial` (`self.StaticMesh`) 0 (`self.OnMaterial`))
  (`PrimitiveComponent.SetCollisionEnabled` (`self.StaticMesh`) "QueryAndPhysics"))

(event `/Game/RhythmGame/Blueprints/Interfaces/BPI_BlinkingPlatform.Invisible`
  (`PrimitiveComponent.SetMaterial` (`self.StaticMesh`) 0 (`self.OffMaterial`))
  (`PrimitiveComponent.SetCollisionEnabled` (`self.StaticMesh`) "NoCollision"))

(fn `UserConstructionScript`)