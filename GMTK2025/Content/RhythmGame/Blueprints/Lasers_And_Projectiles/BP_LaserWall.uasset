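; BP_LaserWall is a rhythm-game hazard wall that switches on and off with instrument clock input and respawns the player on contact.
; RecieveClockInput compares instrument types as strings, then toggles the static mesh's visibility and the actor's collision from the On flag.
; When the player pawn begins overlapping the Box, it finds BP_SpawnManager with GetActorOfClass and calls SpawnPlayer.
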(event `self.ReceiveBeginPlay`)

(event `/Game/RhythmGame/Blueprints/Interfaces/BPI_PlatformFunctionality.RecieveClockInput`
  (params (InstrumentType :type "/Game/RhythmGame/Blueprints/Enumeration/E_InstrumentType Enum" :default "NewEnumerator0") (`On?` :type Boolean))
  (if (`KismetStringLibrary.EqualEqual_StrStr` (`|GetEnumeratorNameAsString` InstrumentType) (`|GetEnumeratorNameAsString` (`self.Instrument Type`)))
    (if `On?`
      (`SceneComponent.SetVisibility` (`self.StaticMesh`) true false)
      (`self.SetActorEnableCollision` true)
      (else
        (`SceneComponent.SetVisibility` (`self.StaticMesh`) false false)
        (`self.SetActorEnableCollision` false)))))

(event `self.Box.OnComponentBeginOverlap`
  (params (OverlappedComponent :type "PrimitiveComponent Object Reference") (OtherActor :type "Actor Object Reference") (OtherComp :type "PrimitiveComponent Object Reference") (OtherBodyIndex :type Integer) (bFromSweep :type Boolean) (SweepResult :type "HitResult Structure (by ref)"))
  (if (== OtherActor (`GameplayStatics.GetPlayerPawn` 0))
    (bind _returnvalue (`GameplayStatics.GetActorOfClass` "/Game/RhythmGame/Blueprints/Spawning/BP_SpawnManager.BP_SpawnManager_C"))
    (`/Game/RhythmGame/Blueprints/Spawning/BP_SpawnManager.SpawnPlayer` _returnvalue)))

(fn `UserConstructionScript`)