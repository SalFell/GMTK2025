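; BP_Emitter is a rhythm-game emitter that fires BP_Projectile actors in response to clock input for its instrument type.
; RecieveClockInput filters on instrument type and, when On is true, spawns a projectile at the FiringDirection component's transform with itself as owner.
; It then sets the projectile movement's initial and max speed to ProjectileSpeed.
; BeginPlay stores start and Distance-offset end locations, which these graphs never use.
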(event `self.ReceiveBeginPlay`
  (set `self.Start Location` (`SceneComponent.K2_GetComponentLocation` (`self.DefaultSceneRoot`)))
  (set `self.End Location` (+ (`self.Start Location`) (`self.Distance`))))

(event `/Game/RhythmGame/Blueprints/Interfaces/BPI_PlatformFunctionality.RecieveClockInput`
  (params (InstrumentType :type "/Game/RhythmGame/Blueprints/Enumeration/E_InstrumentType Enum" :default "NewEnumerator0") (`On?` :type Boolean))
  (bind _projectile_speed (`self.Projectile Speed`))
  (if (`|EnumEquality` InstrumentType (`self.Instrument Type`))
    (if `On?`
      (bind _returnvalue (`|SpawnActorFromClass` "/Game/RhythmGame/Blueprints/Lasers_And_Projectiles/BP_Projectile.BP_Projectile_C" (`SceneComponent.K2_GetComponentToWorld` (`self.Firing_Direction`)) "Undefined" "MultiplyWithRoot" self null))
      (bind _projectilemovement (`/Game/RhythmGame/Blueprints/Lasers_And_Projectiles/BP_Projectile.ProjectileMovement` _returnvalue))
      (set `ProjectileMovementComponent.InitialSpeed` _projectile_speed _projectilemovement)
      (set `ProjectileMovementComponent.MaxSpeed` _projectile_speed _projectilemovement))))

(fn `UserConstructionScript`)