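; Quartz template Blueprint for the rhythm game that plays a kick drum sound in sync with a musical clock.
; On BeginPlay it creates a 4/4 clock at a fixed tempo, subscribes to bar events and queues the sound quantized to the bar.
; The clock starts once, when playback first reports Queued.
; Bar events print the count and, at NumofBars, requeue the sound and reset the transport on a bar boundary to loop.
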(event `self.ReceiveBeginPlay`
  ; Setup Quartz Clock
  (bind _returnvalue (`QuartzSubsystem.CreateNewClock` (subsystem `QuartzSubsystem`) "QuartzMaster" (make `QuartzClockSettings` (make `QuartzTimeSignature` 4)) false true))
  (bind _output_get (set `self.QuartzClock` _returnvalue))
  (bind _clockhandle (`QuartzClockHandle.SetBeatsPerMinute` :`self` _output_get :`BeatsPerMinute` 120.0))
  (`QuartzClockHandle.SubscribeToQuantizationEvent` _clockhandle "Bar" (`|CreateDelegate` :!event `BarEvents`))
  (`self.QueueMusic`))

(event `QueueMusic`
  ; Queue Music
  (bind _returnvalue (`GameplayStatics.CreateSound2D` "/Game/RhythmGame/Audio/KickDrum.KickDrum" 1.0 1.0 0.0 null))
  (`AudioComponent.PlayQuantized` _returnvalue (`self.QuartzClock`) (make `QuartzQuantizationBoundary` "Bar" 1.0 "CurrentTimeRelative") (delegate `CustomEvent_0`) 0.0 0.0 1.0 "Linear"))

(event `BarEvents`
  (params (ClockName :type Name) (QuantizationType :type "EQuartzCommandQuantization Enum" :default "Bar") (NumBars :type Integer) (Beat :type Integer) (BeatFraction :type "Float (single-precision)"))
  ; Count & Retrigger
  (`KismetSystemLibrary.PrintString` (`KismetStringLibrary.Conv_IntToString` NumBars))
  (if (== NumBars (`self.NumofBars`))
    (`self.QueueMusic`)
    (`QuartzClockHandle.ResetTransportQuantized` :`self` (`self.QuartzClock`) :`InQuantizationBoundary` (make `QuartzQuantizationBoundary` "Bar" 1.0 "CurrentTimeRelative"))))

(event `CustomEvent_0`
  (params (EventType :type "EQuartzCommandDelegateSubType Enum" :default "CommandOnFailedToQueue") (Name :type Name))
  ; Queue Music
  (switch `EQuartzCommandDelegateSubType` EventType
    (:`CommandOnQueued`
      (`/Engine/EditorBlueprintResources/StandardMacros.DoOnce` false
        (:`Completed`
          (`QuartzClockHandle.StartClock` (`self.QuartzClock`)))))))

(fn `UserConstructionScript`)