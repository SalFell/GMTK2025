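; BP_Checkpoint is a rhythm-game checkpoint that updates the player's spawn point and switches on an instrument's music track.
; BeginPlay looks up the sequencer track index in DT_PlatformClass by instrument type.
; Player overlap updates the spawn manager, then once, if that instrument is silent, activates all sections of that track in AudioSequenceAmaya.
; It then notifies the first BPI_InstrumentIsOn actor and marks the instrument as playing.
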(event `self.ReceiveBeginPlay`
  (bind _returnvalue (`|GetDataTableRow` "/Game/RhythmGame/Blueprints/Enumeration/DT_PlatformClass.DT_PlatformClass" (`BlueprintMapLibrary.Map_Find` (`self.FolderMap`) (`self.InstrumentType`)))
    (:`then`
      (bind _output_get (set `self.SequencerIndex` (break `/Game/RhythmGame/Blueprints/Enumeration/ST_ClassType` _returnvalue)))
      (`KismetSystemLibrary.PrintString` (`KismetStringLibrary.Conv_IntToString` _output_get))
      (bind _returnvalue_2 (`MovieSceneSequenceExtensions.GetTracks` "/Game/RhythmGame/Audio/AudioSequence.AudioSequence"))
      (`KismetSystemLibrary.PrintString` (`KismetSystemLibrary.GetDisplayName` (`|GetArrayItem` _returnvalue_2 _output_get))))))

(event `self.Box.OnComponentBeginOverlap`
  (params (OverlappedComponent :type "PrimitiveComponent Object Reference") (OtherActor :type "Actor Object Reference") (OtherComp :type "PrimitiveComponent Object Reference") (OtherBodyIndex :type Integer) (bFromSweep :type Boolean) (SweepResult :type "HitResult Structure (by ref)"))
  (bind _spawnpoint (`self.SpawnPoint`))
  (if (== OtherActor (`GameplayStatics.GetPlayerPawn` 0))
    (`/Game/RhythmGame/Blueprints/Spawning/BP_SpawnManager.UpdateSpawnPoint` (`self.SpawnManagerRef`) (`KismetMathLibrary.MakeTransform` (`SceneComponent.K2_GetComponentLocation` _spawnpoint) (`SceneComponent.K2_GetComponentRotation` _spawnpoint)))
    (`/Engine/EditorBlueprintResources/StandardMacros.DoOnce` false
      (:`Completed`
        (if (not (`BlueprintMapLibrary.Map_Find` (`self.InstrumentPlaying?`) (`self.InstrumentType`)))
          ; make sure this is set to the right audio sequencer
          (bind _returnvalue (`MovieSceneSequenceExtensions.GetTracks` "/Game/RhythmGame/LevelSequence/AudioSequenceAmaya.AudioSequenceAmaya"))
          (bind _returnvalue_2 (`MovieSceneTrackExtensions.GetSections` (`|GetArrayItem` _returnvalue (`self.SequencerIndex`))))
          (for _array_element _returnvalue_2
            (`MovieSceneSection.SetIsActive` _array_element true))
          (bind _outactors (`GameplayStatics.GetAllActorsWithInterface` "/Game/RhythmGame/Blueprints/Interfaces/BPI_InstrumentIsOn.BPI_InstrumentIsOn_C"))
          (message `/Game/RhythmGame/Blueprints/Interfaces/BPI_InstrumentIsOn.InstrumentIsOn` (`|GetArrayItem` _outactors) (`self.InstrumentType`))
          (`BlueprintMapLibrary.Map_Add` (`self.InstrumentPlaying?`) (`self.InstrumentType`) true))))))

(fn `UserConstructionScript`)