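; BP_SpawnManager is a rhythm game actor that stores and applies the player's respawn point.
; On BeginPlay it captures the pawn's location and controller rotation as the initial spawn transform.
; UpdateSpawnPoint replaces that transform and prints a confirmation, while SpawnPlayer moves the existing pawn to the saved location and sets the controller's rotation, without spawning a new actor.
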(event `self.ReceiveBeginPlay`
  (set `self.PlayerSpawnPoint` (`KismetMathLibrary.MakeTransform` (`self.K2_GetActorLocation` (`GameplayStatics.GetPlayerPawn` 0)) (`self.K2_GetActorRotation` (`GameplayStatics.GetPlayerController` 0)))))

(event `UpdateSpawnPoint`
  (params (NewSpawn :type "Transform Structure"))
  (set `self.PlayerSpawnPoint` NewSpawn)
  (`KismetSystemLibrary.PrintString` "New Spawn Location Set"))

(event `SpawnPlayer`
  (bind (_playerspawnpoint_location _playerspawnpoint_rotation) (`KismetMathLibrary.BreakTransform` (`self.PlayerSpawnPoint`)))
  (`self.K2_SetActorLocation` (`GameplayStatics.GetPlayerPawn` 0) _playerspawnpoint_location false false)
  (`self.K2_SetActorRotation` (`GameplayStatics.GetPlayerController` 0) _playerspawnpoint_rotation false))

(fn `UserConstructionScript`)