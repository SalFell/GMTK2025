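; BP_Pad is the rhythm game's pad instrument manager, which triggers pad-driven platform movement while the instrument is active.
; ActivateInstrument sets Active when any section of the AudioSongManager track at the KickDrum index, rather than a pad-specific one, is active.
; ExecutePadPlatforms checks that flag, then sends ExecutePlatformMovementMessage with Pad set to every actor implementing BPI_PlatformFunctionality.
; Nothing in this graph clears Active.
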(event `ExecutePadPlatforms`
  (if (`self.Active?`)
    (bind _outactors (`GameplayStatics.GetAllActorsWithInterface` "/Game/RhythmGame/Blueprints/Interfaces/BPI_PlatformFunctionality.BPI_PlatformFunctionality_C"))
    (for _array_element _outactors
      (message `/Game/RhythmGame/Blueprints/Interfaces/BPI_PlatformFunctionality.ExecutePlatformMovement` _array_element false false false false false false true))))

(event `self.ActivateInstrument`
  (bind _audiosongmanagerref (`self.AudioSongManagerRef`))
  (for (_array_element _array_index) (`/Game/RhythmGame/Audio/AudioManagers/BP_AudioSongManager.Tracks` _audiosongmanagerref)
    (if (== _array_index (`/Game/RhythmGame/Audio/AudioManagers/BP_AudioSongManager.KickDrum` _audiosongmanagerref))
      (bind _returnvalue (`MovieSceneTrackExtensions.GetSections` _array_element))
      (for _array_element_2 _returnvalue
        (if (`MovieSceneSection.IsActive` _array_element_2)
          (set `self.Active?` true))))))

(fn `UserConstructionScript`
  (`parent.UserConstructionScript`))