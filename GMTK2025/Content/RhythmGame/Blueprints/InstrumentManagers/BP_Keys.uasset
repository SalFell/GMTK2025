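; BP_Keys is the keys instrument manager in a rhythm game, triggering platform movement tied to that instrument.
; ExecuteKeysPlatforms finds every actor implementing BPI_PlatformFunctionality and sends each a movement message flagged as Keys.
; ActivateInstrument is empty, and the logic to play Audio quantized on the MyQuartz clock's beat is unconnected, so it never runs.
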(event `ExecuteKeysPlatforms`
  (bind _outactors (`GameplayStatics.GetAllActorsWithInterface` "/Game/RhythmGame/Blueprints/Interfaces/BPI_PlatformFunctionality.BPI_PlatformFunctionality_C"))
  (for _array_element _outactors
    (message `/Game/RhythmGame/Blueprints/Interfaces/BPI_PlatformFunctionality.ExecutePlatformMovement` _array_element false false false false false true)))

(event `/Game/RhythmGame/Blueprints/Interfaces/BPI_StartInstrument.ActivateInstrument`
  (params (Quantization :type "EQuartzCommandQuantization Enum" :default "Bar")))

(fn `UserConstructionScript`
  (`parent.UserConstructionScript`))