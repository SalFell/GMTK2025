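; Song manager for a rhythm game that layers music by enabling instrument tracks in AudioSequence.
; BeginPlay caches the tracks and deactivates all sections except those on the kick drum track.
; Start events for hi-hat, clap, lead, keys and brass find their track by index and activate its inactive sections.
; Each activation, kick included, also sends ActivateInstrumentMessage to the matching instrument actor through BPI_StartInstrument.
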(event `self.ReceiveBeginPlay`
  (bind _returnvalue (`MovieSceneSequenceExtensions.GetTracks` "/Game/RhythmGame/LevelSequence/AudioSequence.AudioSequence"))
  (bind _output_get (set `self.Tracks` _returnvalue))
  (for (_array_element _array_index) _output_get
    (bind _returnvalue_2 (`MovieSceneTrackExtensions.GetSections` _array_element))
    (for _array_element_2 _returnvalue_2
      (`MovieSceneSection.SetIsActive` _array_element_2 false)
      (if (== _array_index (`self.KickDrum`))
        (if (not (`MovieSceneSection.IsActive` _array_element_2))
          (`MovieSceneSection.SetIsActive` _array_element_2 true)
          (bind _outactors (`GameplayStatics.GetAllActorsWithInterface` "/Game/RhythmGame/Blueprints/Interfaces/BPI_StartInstrument.BPI_StartInstrument_C"))
          (for _array_element_3 _outactors
            (if (== _array_element_3 (`self.KitDrumRef`))
              (message `/Game/RhythmGame/Blueprints/Interfaces/BPI_StartInstrument.ActivateInstrument` _array_element_3))))))))

(event `StartHiHat`
  (for (_array_element _array_index) (`self.Tracks`)
    (if (== _array_index (`self.HiHat`))
      (bind _returnvalue (`MovieSceneTrackExtensions.GetSections` _array_element))
      (for _array_element_2 _returnvalue
        (if (not (`MovieSceneSection.IsActive` _array_element_2))
          (`MovieSceneSection.SetIsActive` _array_element_2 true)
          (bind _outactors (`GameplayStatics.GetAllActorsWithInterface` "/Game/RhythmGame/Blueprints/Interfaces/BPI_StartInstrument.BPI_StartInstrument_C"))
          (for _array_element_3 _outactors
            (if (== _array_element_3 (`self.HiHatRef`))
              (message `/Game/RhythmGame/Blueprints/Interfaces/BPI_StartInstrument.ActivateInstrument` _array_element_3))))))))

(event `StartClap`
  (for (_array_element _array_index) (`self.Tracks`)
    (if (== _array_index (`self.Clap`))
      (bind _returnvalue (`MovieSceneTrackExtensions.GetSections` _array_element))
      (for _array_element_2 _returnvalue
        (if (not (`MovieSceneSection.IsActive` _array_element_2))
          (`MovieSceneSection.SetIsActive` _array_element_2 true)
          (bind _outactors (`GameplayStatics.GetAllActorsWithInterface` "/Game/RhythmGame/Blueprints/Interfaces/BPI_StartInstrument.BPI_StartInstrument_C"))
          (for _array_element_3 _outactors
            (if (== _array_element_3 (`self.ClapRef`))
              (message `/Game/RhythmGame/Blueprints/Interfaces/BPI_StartInstrument.ActivateInstrument` _array_element_3))))))))

(event `StartLead`
  (for (_array_element _array_index) (`self.Tracks`)
    (if (== _array_index (`self.Lead`))
      (bind _returnvalue (`MovieSceneTrackExtensions.GetSections` _array_element))
      (for _array_element_2 _returnvalue
        (if (not (`MovieSceneSection.IsActive` _array_element_2))
          (`MovieSceneSection.SetIsActive` _array_element_2 true)
          (bind _outactors (`GameplayStatics.GetAllActorsWithInterface` "/Game/RhythmGame/Blueprints/Interfaces/BPI_StartInstrument.BPI_StartInstrument_C"))
          (for _array_element_3 _outactors
            (if (== _array_element_3 (`self.LeadRef`))
              (message `/Game/RhythmGame/Blueprints/Interfaces/BPI_StartInstrument.ActivateInstrument` _array_element_3))))))))

(event `StartKeys`
  (for (_array_element _array_index) (`self.Tracks`)
    (if (== _array_index (`self.Keys`))
      (bind _returnvalue (`MovieSceneTrackExtensions.GetSections` _array_element))
      (for _array_element_2 _returnvalue
        (if (not (`MovieSceneSection.IsActive` _array_element_2))
          (`MovieSceneSection.SetIsActive` _array_element_2 true)
          (bind _outactors (`GameplayStatics.GetAllActorsWithInterface` "/Game/RhythmGame/Blueprints/Interfaces/BPI_StartInstrument.BPI_StartInstrument_C"))
          (for _array_element_3 _outactors
            (if (== _array_element_3 (`self.KeysRef`))
              (message `/Game/RhythmGame/Blueprints/Interfaces/BPI_StartInstrument.ActivateInstrument` _array_element_3))))))))

(event `StartBrass`
  (for (_array_element _array_index) (`self.Tracks`)
    (if (== _array_index (`self.Brass`))
      (bind _returnvalue (`MovieSceneTrackExtensions.GetSections` _array_element))
      (for _array_element_2 _returnvalue
        (if (not (`MovieSceneSection.IsActive` _array_element_2))
          (`MovieSceneSection.SetIsActive` _array_element_2 true)
          (bind _outactors (`GameplayStatics.GetAllActorsWithInterface` "/Game/RhythmGame/Blueprints/Interfaces/BPI_StartInstrument.BPI_StartInstrument_C"))
          (for _array_element_3 _outactors
            (if (== _array_element_3 (`self.BrassRef`))
              (message `/Game/RhythmGame/Blueprints/Interfaces/BPI_StartInstrument.ActivateInstrument` _array_element_3))))))))

(fn `UserConstructionScript`)